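; Enemy respawn volume that keeps a population of Bp_IA AI pawns inside its box.
; A looping timer started on BeginPlay prunes invalid entries from the Enemigos array, then after a delay triggers the respawn check.
; When fewer than four enemies remain, it spawns AI at random points within the Box bounds to bring the count back to eight and tracks them in the array.
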(event `self.ReceiveBeginPlay`
  (bind _output_get (set `self.TiempOleadas` 5.0))
  (`KismetSystemLibrary.K2_SetTimerDelegate` (delegate `RevisarEnemigos`) _output_get true))

(event `RevisarEnemigos`
  (bind (_arrayindex _arrayelement) (`/Engine/EditorBlueprintResources/StandardMacros.ReverseForEachLoop` (`self.Enemigos`))
    (:`LoopBody`
      (`/Engine/EditorBlueprintResources/StandardMacros.IsValid` _arrayelement
        (:`Is Not Valid`
          (`KismetArrayLibrary.Array_Remove` (`self.Enemigos`) _arrayindex))))
    (:`Completed`
      (`KismetSystemLibrary.Delay` 15.0)
      (`self.Respawn Enemigos`))))

(event `Respawn Enemigos`
  (bind _returnvalue (`KismetArrayLibrary.Array_Length` (`self.Enemigos`)))
  (bind (_origin _boxextent) (`KismetSystemLibrary.GetComponentBounds` (`self.Box`)))
  (if (< _returnvalue 4)
    (bind _output_get (set `self.CantidadEnemigos` (- 8 _returnvalue)))
    (for _ (range 1 (+ _output_get 1))
      (bind _returnvalue_2 (`AIBlueprintHelperLibrary.SpawnAIFromClass` "/Game/0_DonClemencio/Characters/Bp_IA.Bp_IA_C" null (`KismetMathLibrary.RandomPointInBoundingBox` _origin _boxextent) (struct) false null))
      (`KismetArrayLibrary.Array_Add` (`self.Enemigos`) _returnvalue_2))))

(fn `UserConstructionScript`)